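; Player skateboarder character that handles pause, location reset, HUD and trick animation on top of its SkateMovementComponent and Score component.
; Input pauses the game with a pause menu, or moves the character to the first PlayerStart found, gated by a DoOnce cooldown.
; Double-jump events play a stylish flip montage on the mesh, locked until it completes or is interrupted.
; BeginPlay adds the HUD, and score updates are only printed to screen.
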(event `EnhancedInput|/Game/SkateBoardGame/Core/Input/Gameplay/IA_Pause`
  (params (ActionValue :type Boolean) (ElapsedSeconds :type "Float (double-precision)") (TriggeredSeconds :type "Float (double-precision)") (InputAction :type "InputAction Object Reference" :default "/Game/SkateBoardGame/Core/Input/Gameplay/IA_Pause.IA_Pause"))
  (:`Started`
    (`GameplayStatics.SetGamePaused` true)
    (bind _returnvalue (`|CreateWidget` "/Game/SkateBoardGame/UI/Widgets/PauseMenu/WB_PauseMenu.WB_PauseMenu_C"))
    (`UserWidget.AddToViewport` _returnvalue 0)))

(event `EnhancedInput|/Game/SkateBoardGame/Core/Input/Gameplay/IA_ResetLocation`
  (params (ActionValue :type Boolean) (ElapsedSeconds :type "Float (double-precision)") (TriggeredSeconds :type "Float (double-precision)") (InputAction :type "InputAction Object Reference" :default "/Game/SkateBoardGame/Core/Input/Gameplay/IA_ResetLocation.IA_ResetLocation"))
  (:`Started`
    (`/Engine/EditorBlueprintResources/StandardMacros.DoOnce` false :!label _label
      (:`Completed`
        (bind _outactors (`GameplayStatics.GetAllActorsOfClass` "/Script/Engine.PlayerStart"))
        (bind (_returnvalue_location _returnvalue_rotation) (`KismetMathLibrary.BreakTransform` (`self.GetTransform` (`|GetArrayItem` _outactors))))
        (`self.K2_SetActorTransform` (`KismetMathLibrary.MakeTransform` _returnvalue_location _returnvalue_rotation))
        (`KismetSystemLibrary.Delay` 10.0)
        (goto _label :!via `Reset`)))))

(event `self.ReceiveBeginPlay`
  (bind _returnvalue (`|CreateWidget` "/Game/SkateBoardGame/UI/Widgets/HUD/W_HUD.W_HUD_C"))
  (`UserWidget.AddToViewport` _returnvalue 0))

(event `self.OnDoubleJump`
  (`/Engine/EditorBlueprintResources/StandardMacros.DoOnce` false :!label _label_2
    (:`Completed`
      (`|PlayMontage` (`self.Mesh`) "/Game/SkateBoardGame/Art/Animations/Skating/Jump/Stylish_Flip_Montage.Stylish_Flip_Montage"
        (:`OnCompleted`
          (goto _label_2 :!via `Reset`))
        (:`OnInterrupted`
          (goto _label_2 :!via `Reset`))))))

(event `self.SkateMovementComponent.OnDoubleJumped`
  (goto _label_2))

(event `self.Score.OnScoreUpdated`
  (params (NewScore :type Integer))
  (`KismetSystemLibrary.PrintString` (`KismetStringLibrary.Conv_IntToString` NewScore)))

(fn `UserConstructionScript`)